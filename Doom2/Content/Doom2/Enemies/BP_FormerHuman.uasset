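; BP_FormerHuman is a Doom 2 Former Human enemy drawn as a Paper2D sprite that copies the player's control rotation, yaw offset 90 degrees, every tick.
; Damage lowers health and briefly swaps the flipbook for a hurt sprite with a pain sound.
; At zero health it plays a death flipbook, disables capsule collision and shifts the sprite's height on a timeline.
; A detection overlap with BP_DoomGuy plays the sight sound once.
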(event OnComponentBeginOverlap(PlayerDetection)
  (params (OverlappedComponent :type Primitive%20Component%20Object%20Reference) (OtherActor :type Actor%20Object%20Reference) (OtherComp :type Primitive%20Component%20Object%20Reference) (OtherBodyIndex :type Integer) (bFromSweep :type Boolean) (SweepResult :type Hit%20Result%20Structure%20%28by%20ref%29))
  (Utilities|Casting|CastToBP_DoomGuy OtherActor)
  (Utilities|FlowControl|DoOnce false
    (:Completed
      (Audio|PlaySound2D "/Game/Doom2/Sounds/A_Cue_FormerHumanSight.A_Cue_FormerHumanSight" 1.0 1.0 0.0 0 0))))

(event EventBeginPlay
  (Variables|Default|SetPlayerPawn (Game|Player|GetPlayerPawn 0)))

(event EventTick
  (params (DeltaSeconds :type Float%20%28single-precision%29))
  (bind _playerpawn (Variables|Default|GetPlayerPawn))
  (bind _returnvalue (Pawn|GetControlRotation _playerpawn :!class /Script/Engine.Pawn))
  (Transformation|SetWorldRotation (Variables|Default|GetFB_FormerHuman) (Math|Rotator|MakeRotator (.roll _returnvalue) (.pitch _returnvalue) (+ (.yaw _returnvalue) 9e+01)) false false))

(event EventDamage
  (params (Damage :type Integer))
  (bind _fb_formerhuman (Variables|Default|GetFB_FormerHuman))
  (bind _fb_formerhuman_2 (Variables|Default|GetFB_FormerHuman))
  (bind _output_get (Variables|Default|SetHealth (- (Variables|Default|GetHealth) Damage)))
  (if (<= _output_get 0)
    (Components|Timeline|SetLooping _fb_formerhuman false)
    (Sprite|SetFlipbook _fb_formerhuman "/Game/Doom2/Enemies/SPR_FormerHuman_Death.SPR_FormerHuman_Death")
    (Audio|PlaySound2D "/Game/Doom2/Sounds/A_Cue_FormerHumanDeath.A_Cue_FormerHumanDeath" 1.0 1.0 0.0 0 0)
    (Collision|SetCollisionEnabled (Variables|Default|GetCapsule) "NoCollision")
    (Collision|SetCollisionResponsetoChannel (Variables|Default|GetFB_FormerHuman) "ECC_Pawn" "ECR_Ignore")
    (bind _alpha (Timeline|Death PlayFromStart)
      (:Update
        (Transformation|SetRelativeLocation _fb_formerhuman_2 (Math|Vector|MakeVector 0.0 0.0 (Math|Float|Lerp (.z (Variables|/Script/Engine.SceneComponent|GetRelativeLocation _fb_formerhuman_2)) 25.0 _alpha)) false false)))
    (else
      (Development|SetHiddeninGame (Variables|Default|GetFB_FormerHuman) true false)
      (Development|SetHiddeninGame (Variables|Default|GetHurtSprite) false false)
      (Audio|PlaySound2D "/Game/Doom2/Sounds/SW_FormerHuman_Hurt.SW_FormerHuman_Hurt" 1.0 1.0 0.0 0 0)
      (Utilities|FlowControl|RetriggerableDelay 0.5)
      (Development|SetHiddeninGame (Variables|Default|GetHurtSprite) true false)
      (Development|SetHiddeninGame (Variables|Default|GetFB_FormerHuman) false false))))

(fn ConstructionScript)